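; Game mode for the Boss 2 level that shows a game over screen when the player dies.
; On BeginPlay it binds to the player character's destroyed event.
; When that fires, it fades the camera to black, creates the Boss 2 game over widget, gives it input focus and pauses the game.
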(event `self.ReceiveBeginPlay`
  (add `self.OnDestroyed` (`GameplayStatics.GetPlayerCharacter` 0) (delegate `ShowUI`)))

(event `ShowUI` :!signature `self.OnDestroyed`
  (params (DestroyedActor :type "Actor Object Reference"))
  (bind _returnvalue (`GameplayStatics.GetPlayerController` 0))
  (`KismetSystemLibrary.Delay` 0.01)
  (`/Engine/EditorBlueprintResources/StandardMacros.IsValid` self
    (:`Is Valid`
      (`PlayerCameraManager.StartCameraFade` :`self` (`GameplayStatics.GetPlayerCameraManager` 0) :`ToAlpha` 1.0 :`Duration` 2.0 :`bHoldWhenFinished` true)
      (`KismetSystemLibrary.Delay` 2.0)
      (bind _returnvalue_2 (`|CreateWidget` "/Game/ThirdPerson/UI/WBP_Boss_2_GameOver.WBP_Boss_2_GameOver_C" _returnvalue))
      (bind _output_get (set `self.Widget_ref` _returnvalue_2))
      (`UserWidget.AddToViewport` _output_get 0)
      (`WidgetBlueprintLibrary.SetInputMode_GameAndUIEx` _returnvalue (`self.Widget_ref`) "DoNotLock" false)
      (`GameplayStatics.SetGamePaused` true))))

(fn `UserConstructionScript`)